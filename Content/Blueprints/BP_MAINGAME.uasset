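; Main controller for a Paper2D Snake game that spawns the HUD, snake head, food and border walls on a 100-unit grid.
; Tick runs through a shrinking Delay as the step timer, checking wall, self and food hits by location comparison rather than physics.
; Food adds score, growth and speed, while WASD gates allow one turn per step and segments follow their predecessor.
; Death flashes sprites and shows game over, then Space reloads the level.
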(event `Spawn new snake part`
  (params (SpawnLocation :type "Vector Structure") (`IS Head` :type Boolean))
  ;[1 1 1] Spawn New Snake Part
  (bind _returnvalue (`|SpawnActorFromClass` "/Game/Blueprints/BP_SNakeBodyPart.BP_SNakeBodyPart_C" (`KismetMathLibrary.MakeTransform` SpawnLocation) "AlwaysSpawn" "OverrideRootScale" null null))
  (`PaperFlipbookComponent.SetFlipbook` (`/Game/Blueprints/BP_SNakeBodyPart.PaperFlipbook` _returnvalue) (select `bool` `IS Head` :`false` "/Game/Flipbooks/YellowSquare_Flipbook.YellowSquare_Flipbook" :`true` "/Game/Flipbooks/RedSquare_Flipbook.RedSquare_Flipbook" :!type "PaperFlipbook Object Reference"))
  (`KismetArrayLibrary.Array_Add` (`self.SankePartsArray`) _returnvalue)
  (set `/Game/Blueprints/BP_SNakeBodyPart.Is Head` `IS Head` _returnvalue)
  (`self.K2_SetActorRotation` _returnvalue (`KismetMathLibrary.MakeRotator` 0.0 (select `int` (`KismetMathLibrary.RandomInteger` 3) :`0` 0.0 :`1` 90.0 :`2` 180.0 :`3` 270.0 :!type "Float (single-precision)")) false))

(event `Spawn Food`
  (bind _returnvalue (- (`self.X_Max`) 100.0))
  (bind _returnvalue_2 (- (`self.Z_Max`) 100.0))
  ;[1 1 1] Spawn Food
  (bind _returnvalue_3 (`|SpawnActorFromClass` "/Game/Blueprints/BpFood.BpFood_C" (`KismetMathLibrary.MakeTransform` (`KismetMathLibrary.MakeVector` (* (`.ReturnValue` (`KismetMathLibrary.FMod` (`KismetMathLibrary.RandomFloatInRange` (* _returnvalue -1.0) _returnvalue) 100.0)) 100.0) -0.1 (* (`.ReturnValue` (`KismetMathLibrary.FMod` (`KismetMathLibrary.RandomFloatInRange` (* _returnvalue_2 -1.0) _returnvalue_2) 100.0)) 100.0))) "AlwaysSpawn" "OverrideRootScale" null null))
  (set `self.Food Actor REF` _returnvalue_3))

(event `Kill Snake`
  ;[1 1 1] Kill Snake
  (set `self.Is Dead` true)
  (for (_array_element _array_index) (`self.SankePartsArray`)
    (`PaperFlipbookComponent.SetFlipbook` (`/Game/Blueprints/BP_SNakeBodyPart.PaperFlipbook` _array_element) (select `bool` (== _array_index 0) :`false` "/Game/Flipbooks/Beath_Flipbook.Beath_Flipbook" :`true` "/Game/Flipbooks/Blank_Flipbook.Blank_Flipbook" :!type "PaperFlipbook Object Reference")))
  (`KismetSystemLibrary.Delay` 0.5)
  (for _array_element_2 (`self.SankePartsArray`)
    (`PaperFlipbookComponent.SetFlipbook` (`/Game/Blueprints/BP_SNakeBodyPart.PaperFlipbook` _array_element_2) "/Game/Flipbooks/Blank_Flipbook.Blank_Flipbook")))

(event `Update Score`
  (params (value :type Integer))
  ;[1 1 1] Update Score
  (bind _output_get (set `self.Score` (+ value (`self.Score`))))
  (`/Game/Blueprints/Bp_UI.Update score` (`self.HUD REF`) _output_get))

(event `self.ReceiveBeginPlay`
  (bind (_remainder _returnvalue) (`KismetMathLibrary.FMod` (`self.Z_Max`) 50.0))
  (bind (_remainder_2 _returnvalue_2) (`KismetMathLibrary.FMod` (`self.X_Max`) 50.0))
  ;[1 1 1] Initialize event
  (bind _returnvalue_3 (`|CreateWidget` "/Game/Blueprints/Bp_UI.Bp_UI_C"))
  (bind _output_get (set `self.HUD REF` _returnvalue_3))
  (`UserWidget.AddToViewport` _output_get 0)
  (switch `int` (`KismetMathLibrary.RandomInteger` 3)
    (:`0`
      (set `self.Direction X` 1))
    (:`1`
      (set `self.Direction X` -1))
    (:`2`
      (set `self.Direction Z` 1))
    (:`3`
      (set `self.Direction Z` -1)))
  (set `self.Delay` 0.2)
  (`KismetArrayLibrary.Array_Clear` (`self.SankePartsArray`))
  (`self.Spawn new snake part` (0.0 0.0 0.0) true)
  (`self.Spawn Food`)
  (for _index (range (* _returnvalue_2 _returnvalue))
    (bind _returnvalue_4 (/ _index _returnvalue))
    (bind _returnvalue_5 (mod _index _returnvalue))
    (if (or (== _returnvalue_4 0) (== _returnvalue_4 (- _returnvalue_2 1)) (== _returnvalue_5 0) (== _returnvalue_5 (- _returnvalue 1)))
      (bind _returnvalue_6 (`|SpawnActorFromClass` "/Game/Blueprints/BPBlock.BPBlock_C" (`KismetMathLibrary.MakeTransform` (`KismetMathLibrary.MakeVector` (+ (* (`self.X_Max`) -1.0) (* _returnvalue_4 100.0)) 0.0 (+ (* (`self.Z_Max`) -1.0) (* _returnvalue_5 100.0)))) "AdjustIfPossibleButDontSpawnIfColliding" "OverrideRootScale" null null))
      (`KismetArrayLibrary.Array_Add` (`self.Wall Blocks Array`) _returnvalue_6))))

(event `self.ReceiveTick`
  (params (DeltaSeconds :type "Float (single-precision)"))
  (bind _sankepartsarray (`self.SankePartsArray`))
  (if (`self.Is Dead`)
    (`/Engine/EditorBlueprintResources/StandardMacros.Gate` true :!label _label
      (:`Exit`
        (`/Engine/EditorBlueprintResources/StandardMacros.DoOnce` false
          (:`Completed`
            (`Widget.RemoveFromParent` (`self.HUD REF`))
            (bind _returnvalue (`GameplayStatics.GetCurrentLevelName` true))
            (`GameplayStatics.OpenLevel` (`KismetStringLibrary.Conv_StringToName` _returnvalue))))))
    (else
      (`KismetSystemLibrary.Delay` (`self.Delay`))
      (`|ExecutionSequence`
        (:`then_0`
          (for (_array_element _array_index) (`self.SankePartsArray`) :!label _label_2
            (if (!= _array_index 0)
              (if (== (`self.K2_GetActorLocation` _array_element) (`self.K2_GetActorLocation` (`|GetArrayItem` (`self.SankePartsArray`))))
                (`self.Kill Snake`)
                (`/Game/Blueprints/Bp_UI.Game Over` (`self.HUD REF`))
                (`self.Break self collison test loop`))))
          (for _array_element_2 (`self.Wall Blocks Array`) :!label _label_3
            (if (== (`self.K2_GetActorLocation` _array_element_2) (`self.K2_GetActorLocation` (`|GetArrayItem` (`self.SankePartsArray`))))
              (`self.Kill Snake`)
              (`/Game/Blueprints/Bp_UI.Game Over` (`self.HUD REF`))
              (`self.Break wall collision test loop`))))
        (:`then_1`
          (if (not (`self.Is Dead`))
            (`|ExecutionSequence`
              (:`then_0`
                (if (== (`self.K2_GetActorLocation` (`|GetArrayItem` (`self.SankePartsArray`))) (`self.K2_GetActorLocation` (`self.Food Actor REF`)) :`ErrorTolerance` 1.0)
                  (`self.Update Score` (`/Game/Blueprints/BpFood.Score` (`self.Food Actor REF`)))
                  (`self.K2_DestroyActor` (`self.Food Actor REF`))
                  (`self.Spawn new snake part` (`self.K2_GetActorLocation` (`|GetArrayItem` _sankepartsarray (`KismetArrayLibrary.Array_LastIndex` _sankepartsarray))))
                  (`self.Spawn Food`)
                  (set `self.Delay` (`KismetMathLibrary.FClamp` (+ (`self.Delay`) -0.01) 0.075 0.2))))
              (:`then_1`
                (`|ExecutionSequence`
                  (:`then_0`
                    (`/Engine/EditorBlueprintResources/StandardMacros.Gate` true :!label _label_4
                      (:`Exit`
                        (if (and (== (`self.Direction Z`) 0) (`self.Can Change Direction`))
                          (set `self.Direction X` 0)
                          (set `self.Direction Z` 1)
                          (set `self.Can Change Direction` false :!label _label_5)))))
                  (:`then_1`
                    (`/Engine/EditorBlueprintResources/StandardMacros.Gate` true :!label _label_6
                      (:`Exit`
                        (if (and (== (`self.Direction Z`) 0) (`self.Can Change Direction`))
                          (set `self.Direction X` 0)
                          (set `self.Direction Z` -1)
                          (goto _label_5)))))
                  (:`then_2`
                    (`/Engine/EditorBlueprintResources/StandardMacros.Gate` true :!label _label_7
                      (:`Exit`
                        (if (and (== (`self.Direction X`) 0) (`self.Can Change Direction`))
                          (set `self.Direction X` -1)
                          (set `self.Direction Z` 0)
                          (goto _label_5)))))
                  (:`then_3`
                    (`/Engine/EditorBlueprintResources/StandardMacros.Gate` true :!label _label_8
                      (:`Exit`
                        (if (and (== (`self.Direction X`) 0) (`self.Can Change Direction`))
                          (set `self.Direction X` 1)
                          (set `self.Direction Z` 0)
                          (goto _label_5)))))
                  (:`then_4`
                    (for _index (range (`KismetArrayLibrary.Array_Length` (`self.SankePartsArray`)))
                      (bind _returnvalue_2 (- (- (`KismetArrayLibrary.Array_Length` (`self.SankePartsArray`)) 1) _index))
                      (if (`/Game/Blueprints/BP_SNakeBodyPart.Is Head` (`|GetArrayItem` (`self.SankePartsArray`) _returnvalue_2))
                        (bind _output (`|GetArrayItem` (`self.SankePartsArray`) _returnvalue_2))
                        (`self.K2_AddActorWorldOffset` _output (`KismetMathLibrary.MakeVector` (* (`self.Direction X`) 100.0) 0.0 (* (`self.Direction Z`) 100.0)) false false)
                        (else
                          (`self.K2_SetActorLocation` _output (`self.K2_GetActorLocation` (`|GetArrayItem` (`self.SankePartsArray`) (- _returnvalue_2 1))) false false))))
                    (set `self.Can Change Direction` true)))))))))))

(event `Break self collison test loop`
  (goto _label_2 :!via `Break`))

(event `Break wall collision test loop`
  (goto _label_3 :!via `Break`))

(event `Key|SpaceBar`
  (params (Key :type "Key Structure"))
  (:`Pressed`
    (goto _label :!via `Open`)))

(event `Key|W`
  (params (Key :type "Key Structure"))
  (:`Pressed`
    (goto _label_4 :!via `Open`))
  (:`Released`
    (goto _label_4 :!via `Close`)))

(event `Key|S`
  (params (Key :type "Key Structure"))
  (:`Pressed`
    (goto _label_6 :!via `Open`))
  (:`Released`
    (goto _label_6 :!via `Close`)))

(event `Key|D`
  (params (Key :type "Key Structure"))
  (:`Pressed`
    (goto _label_7 :!via `Open`))
  (:`Released`
    (goto _label_7 :!via `Close`)))

(event `Key|A`
  (params (Key :type "Key Structure"))
  (:`Pressed`
    (goto _label_8 :!via `Open`))
  (:`Released`
    (goto _label_8 :!via `Close`)))

(fn `UserConstructionScript`)